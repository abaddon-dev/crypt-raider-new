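; Hooded statue interactive object for Level 1, built to turn toward the player.
; BeginPlay caches the player, and a polling event calls FacePlayer within range, which interpolates yaw through a self-repeating short Delay loop.
; Nothing live starts that polling: Tick and PickUp are empty.
; The rotation trigger, grab-related collider adjustment, audio and component destruction sit in disconnected nodes, alongside leftover debug prints.
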(event `self.ReceiveBeginPlay`
  (`parent.ReceiveBeginPlay`)
  (bind _asbp_player (cast `/Game/FirstPerson/BP_Player` (`GameplayStatics.GetPlayerCharacter` 0)))
  (set `self.Char REF BP_Player` _asbp_player))

(event `Face Player`
  (bind (_returnvalue_roll _returnvalue_pitch _returnvalue_yaw) (`KismetMathLibrary.BreakRotator` (`KismetMathLibrary.RInterpTo` (`self.K2_GetActorRotation`) (`KismetMathLibrary.FindLookAtRotation` (`self.K2_GetActorLocation`) (`self.K2_GetActorLocation` (`self.Char REF BP_Player`))) (`GameplayStatics.GetWorldDeltaSeconds`) 20.0)))
  ;[1 1 1] Face player
  (if (`self.Should Rotate?`)
    (`KismetSystemLibrary.PrintString` "TRUE")
    (`self.K2_SetActorRotation` (`KismetMathLibrary.MakeRotator` 0.0 0.0 _returnvalue_yaw))
    (`KismetSystemLibrary.Delay` 0.001)
    (`KismetSystemLibrary.PrintString` "Face Player False 2")
    (`self.Face Player`)
    (else
      (`KismetSystemLibrary.PrintString` "Face Player False 1"))))

(event `Should Rotate Event`
  ;[1 1 1] Check Should Rotate
  (if (<= (`self.GetDistanceTo` (`self.Char REF BP_Player`)) 500.0)
    (`self.Face Player`))
  (`KismetSystemLibrary.Delay` 0.001)
  (`self.Should Rotate Event`))

(event `self.ReceiveTick`
  (params (DeltaSeconds :type "Float (single-precision)")))

(event `/Game/BPI_Items.PickUp`)

(fn `UserConstructionScript`
  (`parent.UserConstructionScript`))