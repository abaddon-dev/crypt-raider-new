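; BP_Axe_Unlock_2 is a Level 1 interactive axe item, derived from a parent Blueprint, that caches the player character on BeginPlay.
; A self-repeating FacePlayer event smoothly yaws it toward the player, but only disconnected code calls it.
; PickUp and overlap events are empty.
; Collider repositioning and resizing, audio playback and component destruction are also left unwired, so the axe adds little live behavior of its own.
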(event `self.ReceiveBeginPlay`
  (`parent.ReceiveBeginPlay`)
  (bind _asbp_player (cast `/Game/FirstPerson/BP_Player` (`GameplayStatics.GetPlayerCharacter` 0)))
  (set `self.Char REF` _asbp_player))

(event `FacePlayer`
  (bind (_returnvalue_roll _returnvalue_pitch _returnvalue_yaw) (`KismetMathLibrary.BreakRotator` (`KismetMathLibrary.RInterpTo` (`self.K2_GetActorRotation`) (`KismetMathLibrary.FindLookAtRotation` (`self.K2_GetActorLocation`) (`self.K2_GetActorLocation` (`self.Char REF`))) (`GameplayStatics.GetWorldDeltaSeconds`) 20.0)))
  ;[1 1 1] Face player
  (`self.K2_SetActorRotation` (`KismetMathLibrary.MakeRotator` 0.0 0.0 _returnvalue_yaw))
  (`KismetSystemLibrary.Delay` 0.001)
  (`self.Face Player`))

(event `self.ReceiveTick`
  (params (DeltaSeconds :type "Float (single-precision)")))

(event `/Game/BPI_Items.PickUp`
  ;[1 1 1] Modyfikacja Box Collider przedmiotu niesionego przez gracza tak, aby nie reagował on z obiektami naprzeciwko. Problem pojawi się wtedy gdy przedmiot zostanie złapany od tyłu. Rozwiązaniem byłoby samoistne przekręcanie się przedmiotu w chwili podniesienia (zmiana Rotation)
)

(event `self.ReceiveActorBeginOverlap`
  (params (OtherActor :type "Actor Object Reference")))

(fn `Face Player`)

(fn `UserConstructionScript`)