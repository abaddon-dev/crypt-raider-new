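; BP_Black_Key is a pickup key that the player collects with the Interact input.
; Box overlap toggles an interaction widget through the ShowInteractionInfo macro, enabling input and opening a Gate for BP_Player on entry, then reversing both on exit.
; Interacting through the open Gate sets HasBlackKey on the player, updates the black key text on KeysHUD and destroys the actor.
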(event `InputAction|Interact`
  (params (Key :type "Key Structure"))
  (:`Pressed`
    (`/Engine/EditorBlueprintResources/StandardMacros.Gate` true :!label _label
      (:`Exit`
        (set `/Game/FirstPerson/BP_Player.HasBlackKey?` true (stale `self.Box.OnComponentBeginOverlap` _asbp_player))
        ;[1 1 1] Dodanie informacji o znalezieniu Black Key
        (bind _askeys_hud (cast `/Game/UI/KeysHUD` (`PlayerController.GetHUD` (`GameplayStatics.GetPlayerController` 0))))
        (`/Game/UI/KeysWidgetBlackKey.UpdateText` (`/Game/UI/KeysHUD.UI_Ref_Black_Key` _askeys_hud))
        (`self.K2_DestroyActor`)))))

(event `self.Box.OnComponentBeginOverlap`
  (params (OverlappedComponent :type "PrimitiveComponent Object Reference") (OtherActor :type "Actor Object Reference") (OtherComp :type "PrimitiveComponent Object Reference") (OtherBodyIndex :type Integer) (bFromSweep :type Boolean) (SweepResult :type "HitResult Structure (by ref)"))
  ;[1 1 1] Show info about usability of interact with item
  (`SceneComponent.SetHiddenInGame` (`self.Widget`) false false)
  (bind _asbp_player (cast `/Game/FirstPerson/BP_Player` OtherActor))
  (`self.EnableInput` (`GameplayStatics.GetPlayerController` 0))
  (goto _label :!via `Open`))

(event `self.Box.OnComponentEndOverlap`
  (params (OverlappedComponent :type "PrimitiveComponent Object Reference") (OtherActor :type "Actor Object Reference") (OtherComp :type "PrimitiveComponent Object Reference") (OtherBodyIndex :type Integer))
  ;[1 1 1] Show info about usability of interact with item
  (`SceneComponent.SetHiddenInGame` (`self.Widget`) true false)
  (cast `/Game/FirstPerson/BP_Player` OtherActor)
  (`self.DisableInput` (`GameplayStatics.GetPlayerController` 0))
  (goto _label :!via `Close`))

(fn `UserConstructionScript`)