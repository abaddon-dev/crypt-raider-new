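; BP_Green_Key is a pickup that grants the player the green key when they press Interact nearby.
; Overlapping its Box with BP_Player enables input and opens a Gate, and leaving disables input and closes it.
; An Interact press through the open Gate sets HasGreenKey on the player, updates the green key text via KeysHUD, and destroys the actor.
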(event `InputAction|Interact`
  (params (Key :type "Key Structure"))
  (:`Pressed`
    (`/Engine/EditorBlueprintResources/StandardMacros.Gate` true :!label _label
      (:`Exit`
        (set `/Game/FirstPerson/BP_Player.Has GreenKey?` true (stale `self.Box.OnComponentBeginOverlap` _asbp_player))
        ;[1 1 1] Dodanie informacji o znalezieniu Black Key
        (bind _askeys_hud (cast `/Game/UI/KeysHUD` (`PlayerController.GetHUD` (`GameplayStatics.GetPlayerController` 0))))
        (`/Game/UI/Keys_Widget_Green_Key.UpdateText` (`/Game/UI/KeysHUD.UI_Ref_Green_Key` _askeys_hud))
        (`self.K2_DestroyActor`)))))

(event `self.Box.OnComponentBeginOverlap`
  (params (OverlappedComponent :type "PrimitiveComponent Object Reference") (OtherActor :type "Actor Object Reference") (OtherComp :type "PrimitiveComponent Object Reference") (OtherBodyIndex :type Integer) (bFromSweep :type Boolean) (SweepResult :type "HitResult Structure (by ref)"))
  (bind _asbp_player (cast `/Game/FirstPerson/BP_Player` OtherActor))
  (`self.EnableInput` (`GameplayStatics.GetPlayerController` 0))
  (goto _label :!via `Open`))

(event `self.Box.OnComponentEndOverlap`
  (params (OverlappedComponent :type "PrimitiveComponent Object Reference") (OtherActor :type "Actor Object Reference") (OtherComp :type "PrimitiveComponent Object Reference") (OtherBodyIndex :type Integer))
  (cast `/Game/FirstPerson/BP_Player` OtherActor)
  (`self.DisableInput` (`GameplayStatics.GetPlayerController` 0))
  (goto _label :!via `Close`))

(fn `UserConstructionScript`
  (`parent.UserConstructionScript`))